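; Spline path actor that defines a route starting at a referenced AI vehicle's location.
; The construction script rebuilds the spline in world space from that location plus the Points array, then prints its length and the vehicle's name.
; It adds a Z-forward spline mesh for each segment, using local positions and tangents to visualize the path.
; BeginPlay is empty, so all logic runs at construction.
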(event EventBeginPlay)

(fn ConstructionScript
  (bind _self self)
  (bind _spline (Variables|Default|GetSpline))
  (bind _output_get (Variables|Default|SetPointsIncludingAILocation (Utilities|Array|MakeArray (Transformation|GetActorLocation (Variables|Default|GetAIVehicleType)))))
  (Utilities|Array|AppendArray _output_get (Variables|Default|GetPoints))
  (Spline|SetSplinePoints (Variables|Default|GetSpline) (Variables|Default|GetPointsIncludingAILocation) "World" true)
  (Development|PrintString (Utilities|String|Append (Utilities|String|ToString(Float) (Spline|GetSplineLength (Variables|Default|GetSpline _self))) "/" (Utilities|GetDisplayName (Variables|Default|GetAIVehicleType _self))))
  (for _index (range 0 (- (Spline|GetNumberOfSplinePoints (Variables|Default|GetSpline)) 2))
    (bind _returnvalue (AddComponent|AddSplineMeshComponent false))
    (SplineMesh|SetForwardAxis _returnvalue "Z" true)
    (SplineMesh|SetStartandEnd _returnvalue (Spline|GetLocationatSplinePoint _spline _index "Local") (Spline|GetTangentatSplinePoint _spline _index "Local") (Spline|GetLocationatSplinePoint _spline (+ _index 1) "Local") (Spline|GetTangentatSplinePoint _spline (+ _index 1) "Local") true :!class /Script/Engine.SplineMeshComponent)))